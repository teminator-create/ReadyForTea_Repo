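; Teapot_BP is a collectable teapot that the player picks up by pressing E while nearby.
; Its Sphere overlap events enable input on the actor when ThirdPersonCharacter1 enters and disable it on exit.
; Pressing E decrements CollectablesLeft on ThirdPersonGameMode, adds a newly created CollectiblesWidget to the viewport, then destroys the actor.
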(event `Key|E`
  (params (Key :type "Key Structure"))
  (:`Pressed`
    (bind _asthird_person_game_mode (cast `/Game/ThirdPersonBP/Blueprints/ThirdPersonGameMode` (`GameplayStatics.GetGameMode`)))
    (bind _result (`/Engine/EditorBlueprintResources/StandardMacros.DecrementInt` (`/Game/ThirdPersonBP/Blueprints/ThirdPersonGameMode.Collectables Left` _asthird_person_game_mode))
      (:`  `
        (set `/Game/ThirdPersonBP/Blueprints/ThirdPersonGameMode.Collectables Left` _result _asthird_person_game_mode)
        (bind _returnvalue (`|CreateWidget` "/Game/Blueprints_KJ/CollectiblesWidget.CollectiblesWidget_C"))
        (`UserWidget.AddToViewport` _returnvalue 0)
        (`self.K2_DestroyActor`)))))

(event `self.Sphere.OnComponentBeginOverlap`
  (params (OverlappedComponent :type "PrimitiveComponent Object Reference") (OtherActor :type "Actor Object Reference") (OtherComp :type "PrimitiveComponent Object Reference") (OtherBodyIndex :type Integer) (bFromSweep :type Boolean) (SweepResult :type "HitResult Structure (by ref)"))
  (cast `/Game/ThirdPersonBP/Blueprints/ThirdPersonCharacter1` OtherActor)
  (`self.EnableInput` (`GameplayStatics.GetPlayerController` 0)))

(event `self.Sphere.OnComponentEndOverlap`
  (params (OverlappedComponent :type "PrimitiveComponent Object Reference") (OtherActor :type "Actor Object Reference") (OtherComp :type "PrimitiveComponent Object Reference") (OtherBodyIndex :type Integer))
  (cast `/Game/ThirdPersonBP/Blueprints/ThirdPersonCharacter1` OtherActor)
  (`self.DisableInput` (`GameplayStatics.GetPlayerController` 0)))

(fn `UserConstructionScript`)